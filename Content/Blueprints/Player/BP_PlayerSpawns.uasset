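; BP_PlayerSpawns is a placeable actor that spawns the two local players and sets up their camera.
; The construction script offsets both spawn points along local Y by DistanceFromCenter.
; SpawnPlayers creates each local player, then spawns and possesses a BP_BaseCharacter at its point.
; It then cross-links the characters, passes both and its own location to the Camera, and makes that Player 1's view target.
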(event `self.ReceiveBeginPlay`)

(event `SpawnPlayers`
  (bind (_returnvalue_location _returnvalue_rotation) (`KismetMathLibrary.BreakTransform` (`SceneComponent.K2_GetComponentToWorld` (`self.Player2Spawn`))))
  (bind (_returnvalue_location_2 _returnvalue_rotation_2) (`KismetMathLibrary.BreakTransform` (`SceneComponent.K2_GetComponentToWorld` (`self.Player1Spawn`))))
  ;[1 1 1] Spawn Players
  (`self.SpawnPlayerCharacter` 0 (`KismetMathLibrary.MakeTransform` _returnvalue_location_2 _returnvalue_rotation_2))
  (`self.SpawnPlayerCharacter` 1 (`KismetMathLibrary.MakeTransform` _returnvalue_location _returnvalue_rotation))
  ;[1 1 1] Set Other Player for Each Player
  (set `/Game/Blueprints/Player/BP_BaseCharacter.OtherPlayer` (`self.Player2`) (`self.Player1`))
  (set `/Game/Blueprints/Player/BP_BaseCharacter.OtherPlayer` (`self.Player1`) (`self.Player2`))
  ;[1 1 1] Set Player 1 and Player 2 in Camera
  (set `/Game/Blueprints/BP_FocusCamera.Player 1` (`self.Player1`) (`self.Camera`))
  (set `/Game/Blueprints/BP_FocusCamera.Player 2` (`self.Player2`) (`self.Camera`))
  ;[1 1 1] Set Up Camera
  (set `/Game/Blueprints/BP_FocusCamera.CameraOrigin` (`self.K2_GetActorLocation`) (`self.Camera`))
  (`PlayerController.SetViewTargetWithBlend` (`PlayerState.GetPlayerController` (`Pawn.PlayerState` (`self.Player1`))) (`self.Camera`) 0.0 "VTBlend_Linear" 0.0 false))

(event `SetSpawnDistance`
  ;[1 1 1] Set Spacing Between Players at Spawn
  (`SceneComponent.K2_SetRelativeLocation` (`self.Player1Spawn`) (`KismetMathLibrary.MakeVector` 0.0 (* (`self.DistanceFromCenter`) -1.0)) false false)
  (`SceneComponent.K2_SetRelativeLocation` (`self.Player2Spawn`) (`KismetMathLibrary.MakeVector` 0.0 (`self.DistanceFromCenter`)) false false))

(fn `SpawnPlayerCharacter`
  (params (PlayerId :type Integer) (SpawnTransform :type "Transform Structure"))
  (`GameplayStatics.CreatePlayer` PlayerId) ; Create Player Controller Slot
  (bind _returnvalue (`|SpawnActorFromClass` "/Game/Blueprints/Player/BP_BaseCharacter.BP_BaseCharacter_C" SpawnTransform "Undefined" "OverrideRootScale" null (`local.PlayerId`) null)) ; Spawns Player Character
  (`Controller.Possess` (`GameplayStatics.GetPlayerController` (`local.PlayerId`)) _returnvalue) ; Player Controller Possesses Player Character
  ;[1 1 1] Set Variable Player 1 or Player 2
  (if (== (`local.PlayerId`) 0)
    (set `self.Player1` _returnvalue)
    (else
      (set `self.Player2` _returnvalue)))
  (return))

(fn `UserConstructionScript`
  (`self.SetSpawnDistance`))