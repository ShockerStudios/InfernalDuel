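; Spline mesh actor that lays a chosen static mesh along an editable spline, with collision disabled.
; The construction script adds one spline mesh component per segment, attached to the spline and bent with the points' locations and tangents.
; Each segment takes roll and Y/Z scale from its two end points, so the mesh can twist and vary in thickness along the path.
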(fn `UserConstructionScript`
  (locals (NewLocalVar_0 :type "Float (double-precision)" :default 0.0))
  (bind _spline (`self.Spline`))
  (bind _spline_2 (`self.Spline`))
  (for _index (range (+ (- (`SplineComponent.GetNumberOfSplinePoints` _spline) 2) 1))
    (bind _returnvalue (`AddComponent|NODE_AddSplineMeshComponent-0`))
    (`StaticMeshComponent.SetStaticMesh` _returnvalue (`self.StaticMesh`))
    (`SplineMeshComponent.SetForwardAxis` _returnvalue (`self.Forward Axis`) true)
    (`self.K2_AttachToComponent` _spline "None" "KeepRelative" "KeepRelative" "KeepRelative")
    (bind _returnvalue_2 (+ _index 1))
    (`SplineMeshComponent.SetStartAndEnd` _returnvalue (`SplineComponent.GetLocationAtSplinePoint` _spline _index "Local") (`SplineComponent.GetTangentAtSplinePoint` _spline _index "Local") (`SplineComponent.GetLocationAtSplinePoint` _spline _returnvalue_2 "Local") (`SplineComponent.GetTangentAtSplinePoint` _spline _returnvalue_2 "Local") true)
    (`PrimitiveComponent.SetCollisionEnabled` _returnvalue "NoCollision")
    (`SplineMeshComponent.SetStartRoll` _returnvalue (`KismetMathLibrary.DegreesToRadians` (`SplineComponent.GetRollAtSplinePoint` _spline_2 _index "Local")) false)
    (`SplineMeshComponent.SetEndRoll` _returnvalue (`KismetMathLibrary.DegreesToRadians` (`SplineComponent.GetRollAtSplinePoint` _spline_2 _returnvalue_2 "Local")) false)
    (`SplineMeshComponent.SetStartScale` _returnvalue (`KismetMathLibrary.MakeVector2D` (.y (`SplineComponent.GetScaleAtSplinePoint` _spline_2 _index)) (.z (`SplineComponent.GetScaleAtSplinePoint` _spline_2 _index))) false)
    (`SplineMeshComponent.SetEndScale` _returnvalue (`KismetMathLibrary.MakeVector2D` (.y (`SplineComponent.GetScaleAtSplinePoint` _spline_2 _returnvalue_2)) (.z (`SplineComponent.GetScaleAtSplinePoint` _spline_2 _returnvalue_2))) true) ; The mesh is update only on the last change
  ))