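; BP_Stage is a stage actor that hosts a player spawner and a focus camera as child actors and exposes their distance settings.
; The construction script sets the spawner's offset to half the spawn distance, links it to the camera, and passes player and camera distance limits to that camera.
; On BeginPlay it has the spawner apply its spawn distance and spawn players using the maximum player distance.
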(event `self.ReceiveBeginPlay`
  (bind _asbp_player_spawns (cast `/Game/Blueprints/Player/BP_PlayerSpawns` (`ChildActorComponent.ChildActor` (`self.PlayerSpawner`))))
  (`/Game/Blueprints/Player/BP_PlayerSpawns.SetSpawnDistance` _asbp_player_spawns)
  (`/Game/Blueprints/Player/BP_PlayerSpawns.SpawnPlayers` _asbp_player_spawns (`self.PlayerMaxDistance`)))

(fn `UserConstructionScript`
  (bind _asbp_player_spawns (cast `/Game/Blueprints/Player/BP_PlayerSpawns` (`ChildActorComponent.ChildActor` (`self.PlayerSpawner`))))
  (set `/Game/Blueprints/Player/BP_PlayerSpawns.DistanceFromCenter` (/ (`self.PlayerSpawnDistance`) 2.0) _asbp_player_spawns)
  (bind _asbp_focus_camera (cast `/Game/Blueprints/BP_FocusCamera` (`ChildActorComponent.ChildActor` (`self.Camera`))))
  (set `/Game/Blueprints/Player/BP_PlayerSpawns.Camera` _asbp_focus_camera _asbp_player_spawns)
  (set `/Game/Blueprints/BP_FocusCamera.MaxPlayerDistance` (`self.PlayerMaxDistance`) _asbp_focus_camera)
  (set `/Game/Blueprints/BP_FocusCamera.MaxCameraDistance` (`self.CameraMaxDistance`) _asbp_focus_camera)
  (set `/Game/Blueprints/BP_FocusCamera.MinCameraDistance` (`self.CameraMinDistance`) _asbp_focus_camera))