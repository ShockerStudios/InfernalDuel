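; Camera controller Blueprint that keeps two players framed, as in a side-on, shared-screen view.
; BeginPlay makes the referenced Camera the view target, stores its origin, and finds both BP_BaseCharacter players, the second by Id.
; Each Tick centers the camera on the players' Y/Z midpoint and scales its X offset by their horizontal Y separation, with a minimum-distance fallback and no smoothing.
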(event `self.ReceiveBeginPlay`
  ;[0.1875 0.1875 0.1875] Instantiate Player Variables
  (set `self.CameraOrigin` (`self.K2_GetActorLocation` (`self.Camera`)))
  (`PlayerController.SetViewTargetWithBlend` (`GameplayStatics.GetPlayerController` 0) (`self.Camera`) 0.0 "VTBlend_Linear" 0.0 false)
  (set `self.Player 1` (cast `/Game/Blueprints/Player/BP_BaseCharacter` (`GameplayStatics.GetPlayerCharacter` 0) :!pure true))
  (bind _outactors (`GameplayStatics.GetAllActorsOfClass` "/Game/Blueprints/Player/BP_BaseCharacter.BP_BaseCharacter_C"))
  (for _array_element _outactors
    (if (== (`/Game/Blueprints/Player/BP_BaseCharacter.id` _array_element) 1)
      (set `self.Player 2` _array_element))))

(event `self.ReceiveTick`
  (params (DeltaSeconds :type "Float (single-precision)"))
  (bind _cameraorigin_x (`KismetMathLibrary.BreakVector` (`self.CameraOrigin`)))
  (bind (_returnvalue_x _returnvalue_y _returnvalue_z) (`KismetMathLibrary.BreakVector` (`self.K2_GetActorLocation` (`self.Player 1`))))
  (bind (_returnvalue_x_2 _returnvalue_y_2 _returnvalue_z_2) (`KismetMathLibrary.BreakVector` (`self.K2_GetActorLocation` (`self.Player 2`))))
  (bind (_returnvalue_x_3 _returnvalue_y_3) (`KismetMathLibrary.BreakVector` (`self.K2_GetActorLocation` (`self.Player 1`))))
  (bind (_returnvalue_x_4 _returnvalue_y_4) (`KismetMathLibrary.BreakVector` (`self.K2_GetActorLocation` (`self.Player 2`))))
  (bind _returnvalue (+ (* (`self.MaxCameraDistance`) (/ (`KismetMathLibrary.Abs` (- _returnvalue_y_3 _returnvalue_y_4)) (`self.MaxPlayerSpace`))) _cameraorigin_x))
  ;[0.3385 0.3385 0.3385] Position Camera Between Both Players
  (if (>= _returnvalue (`self.MinCameraDistance`))
    (set `self.TargetDistance` _returnvalue)
    (else
      (set `self.TargetDistance` (+ (`self.MinCameraDistance`) _cameraorigin_x))))
  (`self.K2_SetActorLocation` (`self.Camera`) (`KismetMathLibrary.MakeVector` (`self.TargetDistance`) (/ (+ _returnvalue_y _returnvalue_y_2) 2.0) (/ (+ _returnvalue_z _returnvalue_z_2) 2.0)) false false))

(fn `UserConstructionScript`)