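; BP_FocusCamera is a two-player camera that keeps itself centred between Player1 and Player2 every Tick.
; It scales its X distance linearly from the players' Y separation relative to MaxPlayerDistance, between minimum and maximum camera distances, offset from CameraOrigin.
; It takes Y and Z from the players' midpoint plus a height offset, then moves there directly.
; The distance is not clamped, so it exceeds the maximum when players separate beyond MaxPlayerDistance.
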(event `self.ReceiveTick`
  (params (DeltaSeconds :type "Float (single-precision)"))
  (bind _cameraorigin_x (`KismetMathLibrary.BreakVector` (`self.CameraOrigin`)))
  ;[0.3385 0.3385 0.3385] Position Camera Between Both Players
  ;;[1 1 1] If TargetDistance is greater than MinCameraDistance, use Target Distance
  (set `self.NewCameraDistance` (+ (`self.CalculateTargetCameraDistance`) _cameraorigin_x))
  (`self.K2_SetActorLocation` self (`self.CalculateCameraLocation`) false false) ; Set Camera Position
)

(fn `CalculateCameraLocation`
  (returns (ReturnValue :type "Vector Structure"))
  (bind (_returnvalue_x _returnvalue_y _returnvalue_z) (`KismetMathLibrary.BreakVector` (`self.K2_GetActorLocation` (`self.Player 1`))))
  (bind (_returnvalue_x_2 _returnvalue_y_2 _returnvalue_z_2) (`KismetMathLibrary.BreakVector` (`self.K2_GetActorLocation` (`self.Player 2`))))
  (return (`KismetMathLibrary.MakeVector` (`self.NewCameraDistance`) (/ (+ _returnvalue_y _returnvalue_y_2) 2.0) (+ (/ (+ _returnvalue_z _returnvalue_z_2) 2.0) (`self.CameraZOffset`)))))

(fn `CalculateTargetCameraDistance`
  (returns (ReturnValue :type "Float (double-precision)"))
  (bind (_returnvalue_x _returnvalue_y) (`KismetMathLibrary.BreakVector` (`self.K2_GetActorLocation` (`self.Player 1`))))
  (bind (_returnvalue_x_2 _returnvalue_y_2) (`KismetMathLibrary.BreakVector` (`self.K2_GetActorLocation` (`self.Player 2`))))
  (return (+ (* (- (`self.MaxCameraDistance`) (`self.MinCameraDistance`)) (/ (`KismetMathLibrary.Abs` (- _returnvalue_y _returnvalue_y_2)) (`self.MaxPlayerDistance`))) (`self.MinCameraDistance`))))

(fn `UserConstructionScript`)